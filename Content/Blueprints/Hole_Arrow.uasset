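; Hole marker arrow for the golf game that bobs vertically above the current hole.
; Tick plays or reverses the ArrowMovement timeline based on UpDown, which a FlipFlop toggles whenever the timeline finishes.
; Timeline updates place the arrow at the GolfGameMode's ArrowLocArray entry for CurrentHole, adding the curve value to Z.
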(event `self.ReceiveBeginPlay`)

(event `self.ReceiveTick`
  (params (DeltaSeconds :type "Float (single-precision)"))
  (if (`self.Up/Down`)
    (bind (_direction _arrowmovement) (`Timeline|ArrowMovement` :!label _label)
      (:`Update`
        (bind _returnvalue (`GameplayStatics.GetActorOfClass` "/Game/Blueprints/GolfGameMode.GolfGameMode_C"))
        (bind (_x _y _z) (`KismetMathLibrary.BreakVector3f` (`|GetArrayItem` (`/Game/Blueprints/GolfGameMode.Arrow_loc_array` _returnvalue) (`/Game/Blueprints/GolfGameMode.current_hole` _returnvalue))))
        (`SceneComponent.K2_SetWorldLocation` (`self.Arrow`) (`KismetMathLibrary.MakeVector` _x _y (+ _arrowmovement _z)) false false))
      (:`Finished`
        (`/Engine/EditorBlueprintResources/StandardMacros.FlipFlop`
          (:`A`
            (set `self.Up/Down` false))
          (:`B`
            (set `self.Up/Down` true)))))
    (else
      (goto _label :!via `Reverse`))))

(fn `UserConstructionScript`)