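; Golf cup actor that detects the ball going in and celebrates the sink.
; Overlapping the Magnet component nudges a GolfBall_Blueprint toward the cup origin with a single VInterpTo step, applied once per begin overlap rather than every tick.
; Overlapping the Box component activates confetti, destroys the ball and plays applause.
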(event `self.ReceiveBeginPlay`)

(event `self.Magnet.OnComponentBeginOverlap`
  (params (OverlappedComponent :type "PrimitiveComponent Object Reference") (OtherActor :type "Actor Object Reference") (OtherComp :type "PrimitiveComponent Object Reference") (OtherBodyIndex :type Integer) (bFromSweep :type Boolean) (SweepResult :type "HitResult Structure (by ref)"))
  (bind _asgolf_ball_blueprint (cast `/Game/Blueprints/GolfBall_Blueprint` OtherActor))
  (`self.K2_SetActorLocation` _asgolf_ball_blueprint (`KismetMathLibrary.VInterpTo` (`self.K2_GetActorLocation` _asgolf_ball_blueprint) (`self.K2_GetActorLocation`) (`GameplayStatics.GetWorldDeltaSeconds`) 2.0) false false))

(event `self.Box.OnComponentBeginOverlap`
  (params (OverlappedComponent :type "PrimitiveComponent Object Reference") (OtherActor :type "Actor Object Reference") (OtherComp :type "PrimitiveComponent Object Reference") (OtherBodyIndex :type Integer) (bFromSweep :type Boolean) (SweepResult :type "HitResult Structure (by ref)"))
  (bind _asgolf_ball_blueprint (cast `/Game/Blueprints/GolfBall_Blueprint` OtherActor))
  (`ActorComponent.Activate` (`self.Confetti`) false)
  (`self.K2_DestroyActor` _asgolf_ball_blueprint)
  (`AudioComponent.Play` (`self.Applause`) 0.0))

(fn `UserConstructionScript`)