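; Player-controlled golf ball that is aimed with the camera, launched by a click-and-drag shot, and counts strokes.
; Pressing left mouse on a resting ball, detected by location samples a short delay apart, moves the cursor to top-center and shows a flattened camera-forward arrow.
; Mouse yaw keeps aiming while pitch locks.
; On release, cursor Y sets the impulse along the arrow, and drags above a small threshold add a stroke.
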(event `self.ReceiveTick`
  (params (DeltaSeconds :type "Float (single-precision)"))
  (bind _arrow (`self.Arrow`))
  (bind _ispressed (`self.IsPressed`))
  (bind _returnvalue (not _ispressed))
  ;[1 1 1] Tick Function (Checks for tickPower and Displays arrow)
  (`|ExecutionSequence`
    (:`then_0`
      (if (`self.IsPressed`)
        (bind _returnvalue_2 (`WidgetLayoutLibrary.GetMousePositionOnViewport`))
        (bind _output_get (set `self.TickPower` (`.Y` (`KismetMathLibrary.BreakVector2D` _returnvalue_2))))
        (`KismetSystemLibrary.PrintString` (`KismetStringLibrary.Conv_DoubleToString` (`KismetMathLibrary.FClamp` _output_get 0.0 1000.0)))))
    (:`then_1`
      (if _ispressed
        (`SceneComponent.SetHiddenInGame` _arrow _returnvalue false)
        (`self.ArrowSet` (`KismetMathLibrary.MakeVector` (.x (`SceneComponent.GetForwardVector` (`self.Camera`))) (.y (`SceneComponent.GetForwardVector` (`self.Camera`)))))
        (set `ArrowComponent.ArrowLength` 100.0 (`self.Arrow`))
        (else
          (`SceneComponent.SetHiddenInGame` _arrow _returnvalue false))))
    (:`then_2`
      (set `self.Location1` (`SceneComponent.K2_GetComponentLocation` (`self.Sphere`)))
      (`KismetSystemLibrary.Delay` 0.2)
      (set `self.Location2` (`SceneComponent.K2_GetComponentLocation` (`self.Sphere`))))))

(event `Shot Power`
  ;[1 1 1] Shot Power
  (if (not (`self.IsPressed`))
    (bind _returnvalue (`WidgetLayoutLibrary.GetMousePositionOnViewport`))
    (set `self.Power` (* (`KismetMathLibrary.FClamp` (`.Y` (`KismetMathLibrary.BreakVector2D` _returnvalue)) 0.0 1000.0) (`self.PowerMultiplier`)))))

(event `InputAxisKey|MouseY`
  (params (AxisValue :type "Float (single-precision)"))
  ;[1 1 1] Camera
  (if (not (`self.IsPressed`))
    (`self.AddControllerPitchInput` (* AxisValue -1.0))))

(event `ArrowSet`
  (params (Direction :type "Vector Structure") (Power :type "Float (double-precision)"))
  ;[1 1 1] Sets direction of Arrow
  (`SceneComponent.K2_SetWorldRotation` (`self.Arrow`) (`KismetMathLibrary.MakeRotFromX` Direction) false false))

(event `InputAxisKey|MouseX`
  (params (AxisValue :type "Float (single-precision)"))
  ;[1 1 1] Camera
  (`self.AddControllerYawInput` AxisValue))

(event `Key|LeftMouseButton`
  (params (Key :type "Key Structure"))
  (bind _power (`self.Power`))
  (bind _returnvalue (== (`self.Location1`) (`self.Location2`) :`ErrorTolerance` 0.75))
  (bind _returnvalue_2 (`KismetMathLibrary.MakeVector` (.x (`SceneComponent.GetForwardVector` (`self.Arrow`))) (.y (`SceneComponent.GetForwardVector` (`self.Arrow`)))))
  ;[1 1 1] Applying shot power on click
  (:`Pressed`
    (if _returnvalue
      (set `self.PressWhileMoving` true)
      (set `self.IsPressed` true)
      (`|ExecutionSequence`
        (:`then_0`
          (`self.SetMouseCenterOfScreen`))
        (:`then_1`
          (bind _returnvalue_3 (`WidgetLayoutLibrary.GetMousePositionOnViewport`))
          (set `self.Power Up Start Position` _returnvalue_3)))))
  (:`Released`
    (set `self.IsPressed` false)
    (if (`self.PressWhileMoving`)
      (if _returnvalue
        (set `self.PressWhileMoving` false)
        (`|ExecutionSequence`
          (:`then_0`
            (`self.Shot Power`)
            (bind _returnvalue_4 (`WidgetLayoutLibrary.GetMousePositionOnViewport`))
            (set `self.Power Up End Position` _returnvalue_4)
            (`PrimitiveComponent.AddImpulse` (`self.Sphere`) (* _power _returnvalue_2) "None" false)
            (`KismetSystemLibrary.PrintText` (`KismetTextLibrary.Conv_VectorToText` _returnvalue_2))
            (`KismetSystemLibrary.PrintText` (`KismetTextLibrary.Conv_DoubleToText` (`self.Power`) "HalfToEven"))
            (if (not (<= (`self.TickPower`) 10.0))
              (`/Engine/EditorBlueprintResources/StandardMacros.IncrementInt` (`self.StrokeCounter`)
                (:`  `
                  (set `self.TickPower` 0.0)))))
          (:`then_1`
            (set `self.Power` _power)
            (set `self.Power` 0.0)))))))

(event `SetMouseCenterOfScreen`
  (bind _returnvalue (`GameplayStatics.GetPlayerController` 0))
  (bind (_sizex _sizey) (`PlayerController.GetViewportSize` _returnvalue))
  ;[1 1 1] Mouse Center of Screen
  (`PlayerController.SetMouseLocation` _returnvalue (`KismetMathLibrary.FTrunc` (`KismetMathLibrary.Conv_IntToDouble` (/ _sizex 2))) (`KismetMathLibrary.FTrunc` (`KismetMathLibrary.Conv_IntToDouble` (- _sizey _sizey)))))

(fn `UserConstructionScript`)