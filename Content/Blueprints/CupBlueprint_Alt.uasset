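; Golf hole cup Actor that registers a ball dropping in, records the score and celebrates with confetti.
; Any Box overlap increments the level ball's StrokeCounter before the GolfBall_Blueprint cast.
; A successful cast fires confetti, appends the count to GolfGameMode's HoleScore, destroys the ball and stops confetti after a short delay.
; The Magnet overlap is empty, and its apparent VInterpTo ball-pull logic is unconnected.
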(event `self.ReceiveBeginPlay`)

(event `self.Magnet.OnComponentBeginOverlap`
  (params (OverlappedComponent :type "PrimitiveComponent Object Reference") (OtherActor :type "Actor Object Reference") (OtherComp :type "PrimitiveComponent Object Reference") (OtherBodyIndex :type Integer) (bFromSweep :type Boolean) (SweepResult :type "HitResult Structure (by ref)")))

(event `self.Box.OnComponentBeginOverlap`
  (params (OverlappedComponent :type "PrimitiveComponent Object Reference") (OtherActor :type "Actor Object Reference") (OtherComp :type "PrimitiveComponent Object Reference") (OtherBodyIndex :type Integer) (bFromSweep :type Boolean) (SweepResult :type "HitResult Structure (by ref)"))
  (bind _returnvalue (`GameplayStatics.GetActorOfClass` "/Game/Blueprints/GolfBall_Blueprint.GolfBall_Blueprint_C"))
  (bind _result (`/Engine/EditorBlueprintResources/StandardMacros.IncrementInt` (`/Game/Blueprints/GolfBall_Blueprint.StrokeCounter` _returnvalue))
    (:`  `
      (set `/Game/Blueprints/GolfBall_Blueprint.StrokeCounter` _result _returnvalue)
      (bind _asgolf_ball_blueprint (cast `/Game/Blueprints/GolfBall_Blueprint` OtherActor))
      (`ActorComponent.Activate` (`self.NS_Confetti`) false)
      (bind _returnvalue_2 (`GameplayStatics.GetActorOfClass` "/Game/Blueprints/GolfGameMode.GolfGameMode_C"))
      (`KismetArrayLibrary.Array_Add` (`/Game/Blueprints/GolfGameMode.HoleScore` _returnvalue_2) (`/Game/Blueprints/GolfBall_Blueprint.StrokeCounter` _asgolf_ball_blueprint))
      (`self.K2_DestroyActor` _asgolf_ball_blueprint)
      (`KismetSystemLibrary.Delay` 1.0)
      (`ActorComponent.Deactivate` (`self.NS_Confetti`)))))

(fn `UserConstructionScript`)