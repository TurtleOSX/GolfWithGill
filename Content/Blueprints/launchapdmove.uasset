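; Moving launch pad that shuttles along X and kicks the golf ball upward when it enters the Box trigger.
; The Osc timeline starts on BeginPlay and adds a relative X offset to the root every update.
; On overlap, the Move timeline raises Bump and applies an impulse slightly below the ball's center each update.
; The impulse is the Z component of a reflection-style vector from ball and Arrow forward vectors, scaled by Magnitude.
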(event `self.ReceiveBeginPlay`
  (bind (_direction _newtrack_0) (`Timeline|Osc`)
    (:`Update`
      (`SceneComponent.K2_AddRelativeLocation` (`self.DefaultSceneRoot`) (`KismetMathLibrary.MakeVector` _newtrack_0) false false))))

(event `self.Box.OnComponentBeginOverlap`
  (params (OverlappedComponent :type "PrimitiveComponent Object Reference") (OtherActor :type "Actor Object Reference") (OtherComp :type "PrimitiveComponent Object Reference") (OtherBodyIndex :type Integer) (bFromSweep :type Boolean) (SweepResult :type "HitResult Structure (by ref)"))
  (bind _returnvalue (`SceneComponent.GetForwardVector` (`self.Arrow`)))
  (bind _asgolf_ball_blueprint (cast `/Game/Blueprints/GolfBall_Blueprint` OtherActor))
  (bind (_direction _newtrack_0) (`Timeline|Move` :!via `PlayFromStart`)
    (:`Update`
      (`SceneComponent.K2_SetRelativeLocation` (`self.Bump`) (`KismetMathLibrary.MakeVector` 0.0 0.0 _newtrack_0) false false)
      (`KismetSystemLibrary.PrintText` (`KismetTextLibrary.Conv_VectorToText` (0.0 0.0 0.0)))
      (bind _sphere (`/Game/Blueprints/GolfBall_Blueprint.Sphere` _asgolf_ball_blueprint))
      (bind _returnvalue_2 (`KismetMathLibrary.Normal` (`SceneComponent.GetForwardVector` (`/Game/Blueprints/GolfBall_Blueprint.Sphere` _asgolf_ball_blueprint))))
      (bind (_x _y _z) (`KismetMathLibrary.BreakVector3f` (`SceneComponent.K2_GetComponentLocation` _sphere)))
      (`PrimitiveComponent.AddImpulseAtLocation` _sphere (`KismetMathLibrary.MakeVector` 0.0 0.0 (.z (* (+ _returnvalue_2 (* (* (`KismetMathLibrary.Dot_VectorVector` _returnvalue_2 (`KismetMathLibrary.Normal` _returnvalue)) 2.0) _returnvalue)) (`self.Magnitude`)))) (`KismetMathLibrary.MakeVector` _x _y (- _z 4.0)) "None"))))

(fn `NewFunction_0`)

(fn `UserConstructionScript`)