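; Golf hole cup actor, named as the no-flag variant, that completes a hole when a GolfBall_Blueprint enters its Box trigger.
; On overlap it fires Niagara confetti, appends the ball's stroke count to GolfGameMode's HoleScore, shows a new Scoreboard widget and destroys the ball.
; After a short delay it stops the confetti and removes the scoreboard.
; The Magnet overlap event is empty, and VInterpTo ball-pull logic is left disconnected.
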(event `self.ReceiveBeginPlay`)

(event `self.Magnet.OnComponentBeginOverlap`
  (params (OverlappedComponent :type "PrimitiveComponent Object Reference") (OtherActor :type "Actor Object Reference") (OtherComp :type "PrimitiveComponent Object Reference") (OtherBodyIndex :type Integer) (bFromSweep :type Boolean) (SweepResult :type "HitResult Structure (by ref)")))

(event `self.Box.OnComponentBeginOverlap`
  (params (OverlappedComponent :type "PrimitiveComponent Object Reference") (OtherActor :type "Actor Object Reference") (OtherComp :type "PrimitiveComponent Object Reference") (OtherBodyIndex :type Integer) (bFromSweep :type Boolean) (SweepResult :type "HitResult Structure (by ref)"))
  (bind _asgolf_ball_blueprint (cast `/Game/Blueprints/GolfBall_Blueprint` OtherActor))
  (`ActorComponent.Activate` (`self.NS_Confetti`) false)
  (bind _returnvalue (`GameplayStatics.GetActorOfClass` "/Game/Blueprints/GolfGameMode.GolfGameMode_C"))
  (`KismetArrayLibrary.Array_Add` (`/Game/Blueprints/GolfGameMode.HoleScore` _returnvalue) (`/Game/Blueprints/GolfBall_Blueprint.StrokeCounter` _asgolf_ball_blueprint))
  (bind _returnvalue_2 (`|CreateWidget` "/Game/HUD/Scoreboard.Scoreboard_C"))
  (`UserWidget.AddToViewport` _returnvalue_2 0)
  (`Widget.SetVisibility` _returnvalue_2 "Visible")
  (`self.K2_DestroyActor` _asgolf_ball_blueprint)
  (`KismetSystemLibrary.Delay` 2.5)
  (`ActorComponent.Deactivate` (`self.NS_Confetti`))
  (`Widget.RemoveFromParent` _returnvalue_2))

(fn `UserConstructionScript`)