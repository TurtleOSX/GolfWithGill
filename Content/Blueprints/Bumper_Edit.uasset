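; Bumper Blueprint that knocks the golf ball away when it overlaps the bumper's box.
; On overlap with a GolfBall_Blueprint, it applies an impulse to the ball's sphere along the Arrow component's forward vector, scaled by Magnitude and flattened to the horizontal plane, then prints that vector.
; The Move timeline then replays from the start, driving the Bump component's relative Z for a bump animation.
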(event `self.Box.OnComponentBeginOverlap`
  (params (OverlappedComponent :type "PrimitiveComponent Object Reference") (OtherActor :type "Actor Object Reference") (OtherComp :type "PrimitiveComponent Object Reference") (OtherBodyIndex :type Integer) (bFromSweep :type Boolean) (SweepResult :type "HitResult Structure (by ref)"))
  (bind _returnvalue (`KismetMathLibrary.MakeVector` (.x (* (`KismetMathLibrary.Normal` (`SceneComponent.GetForwardVector` (`self.Arrow`))) (`self.Magnitude`))) (.y (* (`KismetMathLibrary.Normal` (`SceneComponent.GetForwardVector` (`self.Arrow`))) (`self.Magnitude`)))))
  (bind _asgolf_ball_blueprint (cast `/Game/Blueprints/GolfBall_Blueprint` OtherActor))
  (`|ExecutionSequence`
    (:`then_0`
      (`PrimitiveComponent.AddImpulse` (`/Game/Blueprints/GolfBall_Blueprint.Sphere` _asgolf_ball_blueprint) _returnvalue "None" false)
      (`KismetSystemLibrary.PrintString` (`KismetStringLibrary.Conv_VectorToString` _returnvalue)))
    (:`then_1`
      (bind (_direction _newtrack_0) (`Timeline|Move` :!via `PlayFromStart`)
        (:`Update`
          (`SceneComponent.K2_SetRelativeLocation` (`self.Bump`) (`KismetMathLibrary.MakeVector` 0.0 0.0 _newtrack_0) false false))))))

(fn `NewFunction_0`)

(fn `UserConstructionScript`)