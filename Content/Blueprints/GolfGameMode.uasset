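; Game mode for a golf game that handles out-of-bounds recovery and progression from hole to hole.
; Tick records the ball's safe transform while it is nearly still, then restores it and adds a stroke when the ball falls too low.
; Destruction of the player's ball advances the hole, totals the scores, spawns and possesses a new ball, rebinds the destroy event and moves the hole arrow.
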(event `self.ReceiveTick`
  (params (DeltaSeconds :type "Float (single-precision)"))
  (bind _returnvalue (`GameplayStatics.GetActorOfClass` "/Game/Blueprints/GolfBall_Blueprint.GolfBall_Blueprint_C"))
  (if (`KismetSystemLibrary.IsValid` _returnvalue)
    (`|ExecutionSequence`
      (:`then_0`
        (bind _sphere (`/Game/Blueprints/GolfBall_Blueprint.Sphere` _returnvalue))
        (bind (_x _y _z) (`KismetMathLibrary.BreakVector3f` (`SceneComponent.GetComponentVelocity` _sphere)))
        (if (<= (+ (`KismetMathLibrary.Abs` _x) (`KismetMathLibrary.Abs` _y) (`KismetMathLibrary.Abs` _z)) 5.0)
          (bind (_x_2 _y_2 _z_2) (`KismetMathLibrary.BreakVector3f` (`SceneComponent.K2_GetComponentLocation` _sphere)))
          (set `self.Safe Location` (`KismetMathLibrary.MakeVector` _x_2 _y_2 (+ _z_2 3.0)))
          (set `self.Safe Rotation` (`SceneComponent.K2_GetComponentRotation` _sphere))))
      (:`then_1`
        (if (<= (`.Z` (`KismetMathLibrary.BreakVector3f` (`SceneComponent.K2_GetComponentLocation` _sphere))) -300.0)
          (`PrimitiveComponent.SetPhysicsLinearVelocity` _sphere (0.0 0.0 0.0) false "None")
          (`SceneComponent.K2_SetRelativeLocationAndRotation` _sphere (`self.Safe Location`) (`self.Safe Rotation`) false false)
          (`/Engine/EditorBlueprintResources/StandardMacros.IncrementInt` (`/Game/Blueprints/GolfBall_Blueprint.StrokeCounter` _returnvalue)))))))

(event `Respawn`
  (bind _asgolf_ball_blueprint (cast `/Game/Blueprints/GolfBall_Blueprint` (`GameplayStatics.GetPlayerPawn` 0) :!label _label))
  (add `self.OnDestroyed` _asgolf_ball_blueprint (delegate `Score`)))

(event `self.ReceiveBeginPlay`
  (bind _returnvalue (`GameplayStatics.GetActorOfClass` "/Game/Blueprints/Hole_Arrow.Hole_Arrow_C"))
  (`SceneComponent.K2_SetWorldLocation` (`/Game/Blueprints/Hole_Arrow.Arrow` _returnvalue) (`|GetArrayItem` (`self.Arrow_loc_array`) (`self.current_hole`)) false false)
  (goto _label))

(event `Score` :!signature `self.OnDestroyed`
  (params (DestroyedActor :type "Actor Object Reference"))
  (`KismetSystemLibrary.PrintString` "Destroyed")
  (`KismetSystemLibrary.Delay` 0.2)
  (bind _output_get (set `self.current_hole` (+ (`self.current_hole`) 1)))
  (set `self.Total Score` 0)
  (for _array_element (`self.HoleScore`)
    (set `self.Total Score` (+ _array_element (`self.Total Score`))))
  (bind _output (`|GetArrayItem` (`self.spawn_loc_array`) _output_get))
  (`KismetSystemLibrary.PrintText` (`KismetTextLibrary.Conv_TransformToText` _output))
  (bind _returnvalue (`|SpawnActorFromClass` "/Game/Blueprints/GolfBall_Blueprint.GolfBall_Blueprint_C" _output "AdjustIfPossibleButAlwaysSpawn" "OverrideRootScale" null null))
  (`Controller.Possess` (`GameplayStatics.GetPlayerController` 0) _returnvalue)
  (`self.Respawn`)
  (bind _returnvalue_2 (`GameplayStatics.GetActorOfClass` "/Game/Blueprints/Hole_Arrow.Hole_Arrow_C"))
  (`SceneComponent.K2_SetWorldLocation` (`/Game/Blueprints/Hole_Arrow.Arrow` _returnvalue_2) (`|GetArrayItem` (`self.Arrow_loc_array`) (`self.current_hole`)) false false))

(fn `NewFunction_0`)

(fn `UserConstructionScript`)