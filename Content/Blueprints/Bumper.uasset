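; Bumper actor that reacts when a GolfBall_Blueprint overlaps its Box by animating and launching the player.
; The Move timeline offsets the Bump component along local Z.
; On every timeline update, it launches player 0's Character, rather than the overlapping ball, along the Arrow's forward vector scaled by Magnitude.
; Each update also prints that launch velocity as debug text.
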(event `self.Box.OnComponentBeginOverlap`
  (params (OverlappedComponent :type "PrimitiveComponent Object Reference") (OtherActor :type "Actor Object Reference") (OtherComp :type "PrimitiveComponent Object Reference") (OtherBodyIndex :type Integer) (bFromSweep :type Boolean) (SweepResult :type "HitResult Structure (by ref)"))
  (bind _returnvalue (* (`KismetMathLibrary.GetForwardVector` (`SceneComponent.K2_GetComponentRotation` (`self.Arrow`))) (`self.Magnitude`)))
  (bind _asgolf_ball_blueprint (cast `/Game/Blueprints/GolfBall_Blueprint` OtherActor))
  (bind (_direction _newtrack_0) (`Timeline|Move` :!via `PlayFromStart`)
    (:`Update`
      (`SceneComponent.K2_SetRelativeLocation` (`self.Bump`) (`KismetMathLibrary.MakeVector` 0.0 0.0 _newtrack_0) false false)
      (`KismetSystemLibrary.PrintText` (`KismetTextLibrary.Conv_VectorToText` _returnvalue))
      (bind _ascharacter (cast `Character` (`GameplayStatics.GetPlayerPawn` 0)))
      (`Character.LaunchCharacter` _ascharacter _returnvalue false false))))

(fn `NewFunction_0`)

(fn `UserConstructionScript`)