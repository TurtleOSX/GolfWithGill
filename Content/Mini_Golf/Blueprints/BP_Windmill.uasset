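; BP_Windmill is a mini golf windmill that rotates its Part2 and changes Part1's opacity when it is in the camera's view near the ball.
; Each Tick applies pitch rotation, then line-traces forward from the golf ball's camera.
; A hit on any BP_Windmill with the ball near Part1 swaps in an opacity material driven by a timeline.
; When the trace finds no windmill, Part1's normal material returns and the timeline reverses.
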(event `self.ReceiveTick`
  (params (DeltaSeconds :type "Float (single-precision)"))
  (`|ExecutionSequence`
    (:`then_0`
      (`SceneComponent.K2_AddLocalRotation` (`self.Part_2`) (`KismetMathLibrary.MakeRotator` 0.0 (* DeltaSeconds (`self.Rotation_Velocity`))) false false))
    (:`then_1`
      (bind _returnvalue (`GameplayStatics.GetActorOfClass` "/Game/Blueprints/GolfBall_Blueprint.GolfBall_Blueprint_C"))
      (`/Engine/EditorBlueprintResources/StandardMacros.IsValid` _returnvalue
        (:`Is Valid`
          (bind _camera (`/Game/Blueprints/GolfBall_Blueprint.Camera` _returnvalue))
          (bind _returnvalue_2 (`SceneComponent.K2_GetComponentLocation` _camera))
          (bind _outhit (`KismetSystemLibrary.LineTraceSingle` :`Start` _returnvalue_2 :`End` (+ _returnvalue_2 (* (`KismetMathLibrary.GetForwardVector` (`SceneComponent.K2_GetComponentRotation` _camera)) (`KismetMathLibrary.Conv_DoubleToVector` 2000.0))) :`TraceChannel` "TraceTypeQuery1" :`bIgnoreSelf` false))
          (cast `/Game/Mini_Golf/Blueprints/BP_Windmill` (`.HitActor` (`GameplayStatics.BreakHitResult` _outhit))
            (:`then`
              (if (<= (`KismetMathLibrary.VSize` (- (`SceneComponent.K2_GetComponentLocation` (`/Game/Blueprints/GolfBall_Blueprint.Sphere` _returnvalue)) (`SceneComponent.K2_GetComponentLocation` (`self.Part_1`)))) 200.0)
                (`PrimitiveComponent.SetMaterial` (`self.Part_1`) 0 "/Game/Mini_Golf/Materials/M_Windmill_Opacity.M_Windmill_Opacity")
                (bind (_direction _opacity) (`Timeline|Opacity` :!label _label)
                  (:`Update`
                    (`MeshComponent.SetScalarParameterValueOnMaterials` (`self.Part_1`) "Opacity" _opacity)))))
            (:`CastFailed`
              (`PrimitiveComponent.SetMaterial` (`self.Part_1`) 0 "/Game/Mini_Golf/Materials/M_Windmill.M_Windmill")
              (goto _label :!via `Reverse`))))))))

(fn `UserConstructionScript`)